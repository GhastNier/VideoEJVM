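; BP_Counter is a counter Blueprint whose update logic is only partly wired.
; BeginPlay starts a looping one-second timer that calls UpdateNumber, which increments CurrentNumber and then immediately resets it to zero.
; A disconnected branch holds the threshold check that would either clear the timer or write the number to a TextRender, so the display never updates.
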(event Custom|UpdateNumber
  (bind _result (Math|Integer|IncrementInt (Variables|Default|GetCurrentNumber))
    (:%20%20
      (bind _output_get (Variables|Default|SetCurrentNumber 0)))))

(event EventBeginPlay
  (Utilities|Time|SetTimerbyFunctionName 0 "UpdateNumber" 1.0 true))

(event EventTick
  (params (DeltaSeconds :type Float%20%28single-precision%29)))

(fn ConstructionScript)